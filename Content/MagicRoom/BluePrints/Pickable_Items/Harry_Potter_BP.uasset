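; Potion cauldron for the magic room that turns dropped Item_BP ingredients into crafted items.
; Shaker overlaps consume liquids into CurrentCollection and tint the water through dynamic materials, previewing mixes via recipe lookups.
; A catalyst spawns the matching HashDictionary result, while a flask entering Grub becomes the matching filled item.
; Recipes are order-sensitive keys of up to three elements, and failed matches clear the collection.
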(event OnComponentBeginOverlap(Shaker)
  (params (OverlappedComponent :type Primitive%20Component%20Object%20Reference) (OtherActor :type Actor%20Object%20Reference) (OtherComp :type Primitive%20Component%20Object%20Reference) (OtherBodyIndex :type Integer) (bFromSweep :type Boolean) (SweepResult :type Hit%20Result%20Structure%20%28by%20ref%29))
  (bind _currentcollection (Variables|Default|GetcurrentCollection))
  (bind _cotl_water (Variables|Default|Getcotl_water))
  (bind _asitem_bp (Utilities|Casting|CastToItem_BP OtherActor))
  ;[1 1 1] Появление воды
  (if (Utilities|Enum|Equal(Enum) (Variables|/Game/MagicRoom/BluePrints/Pickable_Items/Item_BP.Item_BP_C|Gettype _asitem_bp) "Жидкость")
    (if (Variables|Default|GetiWater?)
      (bind (_newcolor _isfind_) (Utilities|SearchinWater (Variables|/Game/MagicRoom/BluePrints/Pickable_Items/Item_BP.Item_BP_C|Getname _asitem_bp))
        (:Output
          (if _isfind_
            (bind _returnvalue (Rendering|Material|CreateDynamicMaterialInstance _cotl_water 0 "/Game/Assets/Material/MaterialBubl_PotterWater.MaterialBubl_PotterWater" "" :!class /Script/Engine.PrimitiveComponent))
            (Rendering|Material|SetVectorParameterValue _returnvalue "color" (Math|Conversions|ToLinearColor(Color) _newcolor) :!class /Script/Engine.MaterialInstanceDynamic)
            (else
              (bind _returnvalue_2 (Rendering|Material|CreateDynamicMaterialInstance _cotl_water 0 "/Engine/BufferVisualization/BaseColor.BaseColor" "" :!class /Script/Engine.PrimitiveComponent))
              (Rendering|Material|SetVectorParameterValue _returnvalue_2 "color" "(R=0.030000,G=0.000000,B=0.016674,A=1.000000)" :!class /Script/Engine.MaterialInstanceDynamic)))))
      (else
        (Rendering|SetVisibility (Variables|Default|Getcotl_water) true false)
        (Variables|Default|SetiWater? true)
        (Rendering|SetVisibility (Variables|Default|GetParticlBubl) true false)
        (bind _returnvalue_3 (Rendering|Material|CreateDynamicMaterialInstance (Variables|Default|Getcotl_water) 0 "/Game/Assets/Material/MaterialBubl_PotterWater.MaterialBubl_PotterWater" "" :!class /Script/Engine.PrimitiveComponent))
        (Rendering|Material|SetVectorParameterValue _returnvalue_3 "color" (Math|Conversions|ToLinearColor(Color) (Variables|/Game/MagicRoom/BluePrints/Pickable_Items/Item_BP.Item_BP_C|Getrgb _asitem_bp)) :!class /Script/Engine.MaterialInstanceDynamic)))
    (Utilities|Array|Add _currentcollection (Variables|/Game/MagicRoom/BluePrints/Pickable_Items/Item_BP.Item_BP_C|Getname _asitem_bp))
    (Actor|DestroyActor _asitem_bp)
    (for _array_element _currentcollection
      (Development|PrintString _array_element))
    (elif (Utilities|Enum|Equal(Enum) (Variables|/Game/MagicRoom/BluePrints/Pickable_Items/Item_BP.Item_BP_C|Gettype _asitem_bp) "Катализатор")
      (if (Variables|Default|GetiWater?)
        (if (> (Utilities|Array|Length (Variables|Default|GetcurrentCollection)) 0)
          (Utilities|Array|Add (Variables|Default|GetcurrentCollection) (Variables|/Game/MagicRoom/BluePrints/Pickable_Items/Item_BP.Item_BP_C|Gettype _asitem_bp))
          (Actor|DestroyActor _asitem_bp)
          (bind (_result _isfind__2) (Utilities|SearchinDictionary)
            (:Out
              (if _isfind__2
                (Utilities|Array|Clear (Variables|Default|GetcurrentCollection))
                (Rendering|SetVisibility (Variables|Default|Getcotl_water) false false)
                (Rendering|SetVisibility (Variables|Default|GetParticlBubl) false false)
                (Variables|Default|SetiWater? false)
                (bind _returnvalue_4 (Game|SpawnActorfromClass "/Game/MagicRoom/BluePrints/Pickable_Items/Item_BP.Item_BP_C" (Math|Conversions|ToTransform(Vector) (+ (Transformation|GetWorldLocation (Variables|Default|GetDefaultSceneRoot)) "0, 0,30.000000")) "Undefined" 0 0))
                (Variables|/Game/MagicRoom/BluePrints/Pickable_Items/Item_BP.Item_BP_C|Setname _returnvalue_4 (.name (Utilities|Struct|BreakResult _result)))
                (bind _output_get (Variables|/Game/MagicRoom/BluePrints/Pickable_Items/Item_BP.Item_BP_C|Settype _returnvalue_4 (.type (Utilities|Struct|BreakResult _result))))
                (Components|StaticMesh|SetStaticMesh (Variables|/Script/Engine.StaticMeshActor|GetStaticMeshComponent _returnvalue_4) (.MyMesh (Utilities|Struct|BreakResult _result)))
                (if (Utilities|Enum|Equal(Enum) _output_get "Сфера")
                  (bind _output_get_2 (Variables|/Game/MagicRoom/BluePrints/Pickable_Items/Item_BP.Item_BP_C|SetmaterialMain _returnvalue_4 (.materialMain (Utilities|Struct|BreakResult _result))))
                  (Rendering|Material|SetMaterial (Variables|/Script/Engine.StaticMeshActor|GetStaticMeshComponent _returnvalue_4) 0 _output_get_2)
                  ;[1 1 1] ТЕСТОВОЕ
                  (Class|PrimitiveComponent|SetMassOverrideinKg (Variables|/Script/Engine.StaticMeshActor|GetStaticMeshComponent _returnvalue_4) "None" 5.0 true)
                  (Effects|Components|ParticleSystem|SetTemplate (Variables|/Game/MagicRoom/BluePrints/Pickable_Items/Item_BP.Item_BP_C|GetmyParticleSystem _returnvalue_4) (.Particle (Utilities|Struct|BreakResult _result)))
                  (Rendering|SetVisibility (Variables|/Game/MagicRoom/BluePrints/Pickable_Items/Item_BP.Item_BP_C|GetmyParticleSystem _returnvalue_4) true false))
                (else
                  (Utilities|Array|Clear (Variables|Default|GetcurrentCollection))
                  (Variables|Default|SetiWater? false)))))
          (else
            (Actor|DestroyActor _asitem_bp :!label _label)
            (Development|PrintString "BAX")))
        (else
          (goto _label)))
      (else
        (Development|PrintString "Сфера или колба")))))

(event OnComponentBeginOverlap(Grub)
  (params (OverlappedComponent :type Primitive%20Component%20Object%20Reference) (OtherActor :type Actor%20Object%20Reference) (OtherComp :type Primitive%20Component%20Object%20Reference) (OtherBodyIndex :type Integer) (bFromSweep :type Boolean) (SweepResult :type Hit%20Result%20Structure%20%28by%20ref%29))
  (if (Variables|Default|GetiWater?)
    (bind _asitem_bp (Utilities|Casting|CastToItem_BP OtherActor))
    (if (Utilities|Enum|Equal(Enum) (Variables|/Game/MagicRoom/BluePrints/Pickable_Items/Item_BP.Item_BP_C|Gettype _asitem_bp) "Колба")
      (Utilities|Array|Add (Variables|Default|GetcurrentCollection) (Variables|/Game/MagicRoom/BluePrints/Pickable_Items/Item_BP.Item_BP_C|Gettype _asitem_bp))
      (bind (_result _isfind_) (Utilities|SearchinDictionary)
        (:Out
          (if _isfind_
            (Utilities|Array|Clear (Variables|Default|GetcurrentCollection))
            (Variables|/Game/MagicRoom/BluePrints/Pickable_Items/Item_BP.Item_BP_C|Setname _asitem_bp (.name (Utilities|Struct|BreakResult _result)))
            (Variables|/Game/MagicRoom/BluePrints/Pickable_Items/Item_BP.Item_BP_C|Settype _asitem_bp (.type (Utilities|Struct|BreakResult _result)))
            (Rendering|Material|SetMaterial (Variables|/Script/Engine.StaticMeshActor|GetStaticMeshComponent _asitem_bp) 1 (.materialMain (Utilities|Struct|BreakResult _result)))
            (bind _returnvalue (Rendering|Material|CreateDynamicMaterialInstance (Variables|/Script/Engine.StaticMeshActor|GetStaticMeshComponent _asitem_bp) 2 "/Game/Assets/Material/MaterialBubl_PotterWater.MaterialBubl_PotterWater" "" :!class /Script/Engine.PrimitiveComponent))
            (Rendering|Material|SetVectorParameterValue _returnvalue "color" (Math|Conversions|ToLinearColor(Color) (.rgb (Utilities|Struct|BreakResult _result))) :!class /Script/Engine.MaterialInstanceDynamic)
            (Variables|/Game/MagicRoom/BluePrints/Pickable_Items/Item_BP.Item_BP_C|Setrgb _asitem_bp (Math|Conversions|ToColor(LinearColor) (Math|Conversions|ToLinearColor(Color) (.rgb (Utilities|Struct|BreakResult _result)))))
            (Variables|Default|SetiWater? false)
            (Rendering|SetVisibility (Variables|Default|Getcotl_water) false false)
            (Rendering|SetVisibility (Variables|Default|GetParticlBubl) false false)
            (else
              (Utilities|Array|Clear (Variables|Default|GetcurrentCollection))
              (Variables|Default|SetiWater? false)
              (Actor|DestroyActor _asitem_bp)
              (Development|PrintString "BAX"))))))))

(fn ConstructionScript)